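; BP_Mover is a component that moves its owning actor a set distance along a vector, once triggered.
; It records the owner's location at BeginPlay, and OnTriggered sets a flag that enables movement.
; Each Tick adds MoveVector without sweep until the distance from the start reaches MoveDistance, then clears the flag.
; The step is not scaled by delta time, so speed depends on frame rate.
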(event EventBeginPlay
  (Variables|Default|SetStartLocation (Transformation|GetActorLocation (Components|GetOwner))))

(event EventTick
  (params (DeltaSeconds :type Float%20%28single-precision%29))
  (bind _returnvalue (Components|GetOwner))
  (if (Variables|Default|GetbShouldMove)
    (if (>= (Math|Vector|VectorLength (- (Transformation|GetActorLocation (Components|GetOwner)) (Variables|Default|GetStartLocation))) (Variables|Default|GetMove%20Distance))
      (Variables|Default|SetbShouldMove false)
      (else
        (Transformation|SetActorLocation _returnvalue (+ (Transformation|GetActorLocation _returnvalue) (Variables|Default|GetMove%20Vector)) false false)))))

(fn OnTriggered
  (Variables|Default|SetbShouldMove true))