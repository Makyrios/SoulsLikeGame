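; One-shot trigger actor that activates Gruntling enemies when the player walks into it.
; On overlap with an actor tagged as the player, it finds every BP_GruntlingEnemy carrying its TriggerTag and calls PerformSpawn on each, then destroys itself.
; It works on existing tagged instances; a hard-coded SpawnActor node is left disconnected, and a debug "Hello" print remains.
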(event EventBeginPlay)

(event Collision|EventActorBeginOverlap
  (params (OtherActor :type Actor%20Object%20Reference))
  (if (Actor|ActorHasTag OtherActor "Character.Player")
    (Development|PrintString "Hello")
    (bind _outactors (Actor|GetAllActorsOfClasswithTag "/Game/CombatSystem/Enemies/GruntlingEnemy/BP_GruntlingEnemy.BP_GruntlingEnemy_C" (Variables|Default|GetTrigger%20Tag)))
    (for _array_element _outactors
      (Class|MasterAI|PerformSpawn _array_element true))
    (Actor|DestroyActor)))

(event EventTick
  (params (DeltaSeconds :type Float%20%28single-precision%29)))

(fn ConstructionScript)